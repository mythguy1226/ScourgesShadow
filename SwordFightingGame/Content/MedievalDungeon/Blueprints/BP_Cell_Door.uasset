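; BP_Cell_Door is a dungeon cell door that swings open when the knight (BP_KnightController) enters its trigger box.
; The overlap opens it only if it is flagged openable and not yet opened, playing an opening sound at the door.
; A timeline drives the door mesh's relative yaw with a negated curve value, then marks it opened on finish, with no closing logic.
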(event `self.Box.OnComponentBeginOverlap`
  (params (OverlappedComponent :type "PrimitiveComponent Object Reference") (OtherActor :type "Actor Object Reference") (OtherComp :type "PrimitiveComponent Object Reference") (OtherBodyIndex :type Integer) (bFromSweep :type Boolean) (SweepResult :type "HitResult Structure (by ref)"))
  (bind _asbp_knight_controller (cast `/Game/SwordFightingGame/Blueprints/BP_KnightController` OtherActor))
  (`/Engine/EditorBlueprintResources/StandardMacros.IsValid` _asbp_knight_controller
    (:`Is Valid`
      (if (`self.IsOpenable`)
        (if (not (`self.IsOpened`))
          (`GameplayStatics.PlaySoundAtLocation` "/Game/SwordFightingGame/Assets/Sounds/Door_Opening.Door_Opening" (`self.K2_GetActorLocation`) (struct) 1.0 1.0 0.0 null null null null)
          ;[1 1 1] Open the doors and set them to opened after finished
          (bind (_direction _rotate_left_door _rotate_right_door) (`Timeline|Timeline_0`)
            (:`Update`
              (`SceneComponent.K2_SetRelativeRotation` (`self.SM_Cell_Door`) (`KismetMathLibrary.MakeRotator` 0.0 0.0 (* _rotate_right_door -1.0)) false false))
            (:`Finished`
              (set `self.IsOpened` true))))))))

(fn `UserConstructionScript`)